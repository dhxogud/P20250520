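; BP_P38 is a player-controlled plane pawn that constantly flies forward, steers with roll and pitch, boosts and fires rockets.
; Tick feeds its forward vector into FloatingPawnMovement, while axis inputs apply frame-rate-scaled local rotations and Boost swaps acceleration and top speed.
; Fire spawns a short-lived BP_Rocket at the Arrow component's transform.
; BeginPlay registers the Left and Right components with BPSceneRotator; a manual-offset movement alternative sits unused.
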(event EventTick
  (params (DeltaSeconds :type Float%20%28single-precision%29))
  ;[0.15 0.15 0.15 0.5] Using FloatingPawnMovement Version
  (Pawn|Input|AddMovementInput (Transformation|GetActorForwardVector self) 1.0 false))

(event EventBeginPlay
  (Utilities|Array|Add (Variables|/Game/BluePrints/BP_SceneRotator.BP_SceneRotator_C|GetSceneComponents (Variables|Default|GetBP_SceneRotator)) (Variables|Default|GetRight))
  (Utilities|Array|Add (Variables|/Game/BluePrints/BP_SceneRotator.BP_SceneRotator_C|GetSceneComponents (Variables|Default|GetBP_SceneRotator)) (Variables|Default|GetLeft)))

(event Input|ActionEvents|InputActionFire
  (params (Key :type Key%20Structure :default "None"))
  (:Pressed
    (bind _returnvalue (Game|SpawnActorfromClass "/Game/BluePrints/BP_Rocket.BP_Rocket_C" (Transformation|GetWorldTransform (Variables|Default|GetArrow)) "Undefined" "MultiplyWithRoot" (Components|GetOwner) self))
    (Utilities|IsValid _returnvalue
      (:Is%20Valid
        (Actor|SetLifeSpan _returnvalue 3.0)))))

(event Input|ActionEvents|InputActionBoost
  (params (Key :type Key%20Structure :default "None"))
  (bind _floatingpawnmovement (Variables|Default|GetFloatingPawnMovement))
  (bind _floatingpawnmovement_2 (Variables|Default|GetFloatingPawnMovement))
  (:Pressed
    (Variables|/Script/Engine.FloatingPawnMovement|SetAcceleration _floatingpawnmovement_2 4e+03)
    (Variables|/Script/Engine.FloatingPawnMovement|SetMaxSpeed _floatingpawnmovement_2 1.2e+04))
  (:Released
    (Variables|/Script/Engine.FloatingPawnMovement|SetAcceleration _floatingpawnmovement 2e+03)
    (Variables|/Script/Engine.FloatingPawnMovement|SetMaxSpeed _floatingpawnmovement 1.2e+03)))

(event Input|AxisEvents|InputAxisRoll
  (params (AxisValue :type Float%20%28single-precision%29))
  ;[0.15 0.15 0.15 0.5] Roll Rotator
  (Transformation|AddActorLocalRotation (Math|Rotator|MakeRotator (* (Math|Float|Clamp(Float) AxisValue -1.0) (Variables|Default|GetRotSpeed) (Utilities|Time|GetWorldDeltaSeconds)) 0.0 0.0) false false))

(event Input|AxisEvents|InputAxisPitch
  (params (AxisValue :type Float%20%28single-precision%29))
  ;[0.15 0.15 0.15 0.5] Pitch Rotator
  (Transformation|AddActorLocalRotation (Math|Rotator|MakeRotator 0.0 (* (Math|Float|Clamp(Float) AxisValue -1.0) (Variables|Default|GetRotSpeed) (Utilities|Time|GetWorldDeltaSeconds)) 0.0) false false))

(fn ConstructionScript)